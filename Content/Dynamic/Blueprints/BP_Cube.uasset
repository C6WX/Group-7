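; BP_Cube is a box that the third-person character can push and pull around the level.
; Overlaps on the Fwd component toggle the character's CanInteractBox flag.
; While that and IsInteractingBox are true, Tick reads the character's axes and calls SpeedDirection, which interpolates SMCube's relative location along a selected direction vector.
; The right/left check compares RightLeftAxis to itself, so the left branch never runs.
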(event OnComponentBeginOverlap(Fwd)
  (params (OverlappedComponent :type Primitive%20Component%20Object%20Reference) (OtherActor :type Actor%20Object%20Reference) (OtherComp :type Primitive%20Component%20Object%20Reference) (OtherBodyIndex :type Integer) (bFromSweep :type Boolean) (SweepResult :type Hit%20Result%20Structure%20%28by%20ref%29))
  (Development|PrintString "Character can interact")
  (Variables|/Game/Dynamic/ThirdPerson/Blueprints/BP_ThirdPersonCharacter.BP_ThirdPersonCharacter_C|SetCanInteractBox? (Variables|Default|GetCharacterReference) true) ; Sets can interact box to true when the player enters the box collider
)

(event OnComponentEndOverlap(Fwd)
  (params (OverlappedComponent :type Primitive%20Component%20Object%20Reference) (OtherActor :type Actor%20Object%20Reference) (OtherComp :type Primitive%20Component%20Object%20Reference) (OtherBodyIndex :type Integer))
  (Development|PrintString "Character cannot interact")
  (Variables|/Game/Dynamic/ThirdPerson/Blueprints/BP_ThirdPersonCharacter.BP_ThirdPersonCharacter_C|SetCanInteractBox? (Variables|Default|GetCharacterReference) false) ; Sets interact box to false when the player leaves the box collider
)

(event EventTick
  (params (DeltaSeconds :type Float%20%28single-precision%29))
  (bind _characterreference (Variables|Default|GetCharacterReference))
  (bind _right_left_axis (Variables|/Game/Dynamic/ThirdPerson/Blueprints/BP_ThirdPersonCharacter.BP_ThirdPersonCharacter_C|GetRight%20Left%20Axis _characterreference))
  (if (Variables|/Game/Dynamic/ThirdPerson/Blueprints/BP_ThirdPersonCharacter.BP_ThirdPersonCharacter_C|GetIsInteractingBox? (Variables|Default|GetCharacterReference))
    (if (Variables|/Game/Dynamic/ThirdPerson/Blueprints/BP_ThirdPersonCharacter.BP_ThirdPersonCharacter_C|GetCanInteractBox? (Variables|Default|GetCharacterReference))
      (Utilities|FlowControl|Sequence
        (:then_0
          (if (== (Variables|/Game/Dynamic/ThirdPerson/Blueprints/BP_ThirdPersonCharacter.BP_ThirdPersonCharacter_C|GetForward%20Backward%20Axis (Variables|Default|GetCharacterReference)) 0.0)
            (Development|PrintString "Not moving on Forward/Backwards")
            (elif (>= (Variables|/Game/Dynamic/ThirdPerson/Blueprints/BP_ThirdPersonCharacter.BP_ThirdPersonCharacter_C|GetForward%20Backward%20Axis (Variables|Default|GetCharacterReference)) 0.1)
              (Development|PrintString "Is moving forwards")
              (Utilities|Speed/Direction true -2e+01)
              (else
                (Development|PrintString "Is moving backwards")
                (Utilities|Speed/Direction true 2e+01)))))
        (:then_1
          (if (== _right_left_axis 0.0)
            (Development|PrintString "Not moving on Left/Right")
            (elif (>= _right_left_axis (Variables|/Game/Dynamic/ThirdPerson/Blueprints/BP_ThirdPersonCharacter.BP_ThirdPersonCharacter_C|GetRight%20Left%20Axis (Variables|Default|GetCharacterReference)))
              (Development|PrintString "Is moving Right")
              (Utilities|Speed/Direction false 2e+01)
              (else
                (Development|PrintString "Is moving Left")
                (Utilities|Speed/Direction false -2e+01)))))))))

(event EventBeginPlay
  (bind _returnvalue (Actor|GetActorOfClass "/Game/Dynamic/ThirdPerson/Blueprints/BP_ThirdPersonCharacter.BP_ThirdPersonCharacter_C"))
  (Variables|Default|SetCharacterReference _returnvalue))

(fn ConstructionScript)