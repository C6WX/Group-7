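; BP_Diary is a puzzle pickup that grants the player a key once all three codes are held.
; On actor overlap it casts to BP_ThirdPersonCharacter and checks the Code1, Code2 and Code3 flags.
; When all three are true it destroys its Cube1 component, sets the character's Key flag and prints a confirmation message.
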(event Collision|EventActorBeginOverlap
  (params (OtherActor :type Actor%20Object%20Reference))
  (bind _asbp_third_person_character (Utilities|Casting|CastToBP_ThirdPersonCharacter OtherActor))
  (if (Variables|/Game/Dynamic/ThirdPerson/Blueprints/BP_ThirdPersonCharacter.BP_ThirdPersonCharacter_C|GetCode%201 _asbp_third_person_character)
    (if (Variables|/Game/Dynamic/ThirdPerson/Blueprints/BP_ThirdPersonCharacter.BP_ThirdPersonCharacter_C|Getcode2 _asbp_third_person_character)
      (if (Variables|/Game/Dynamic/ThirdPerson/Blueprints/BP_ThirdPersonCharacter.BP_ThirdPersonCharacter_C|Getcode3 _asbp_third_person_character)
        (Components|DestroyComponent (Variables|Default|GetCube1))
        (Variables|/Game/Dynamic/ThirdPerson/Blueprints/BP_ThirdPersonCharacter.BP_ThirdPersonCharacter_C|Setkey _asbp_third_person_character true)
        (Development|PrintText "Key got")))))

(fn ConstructionScript)